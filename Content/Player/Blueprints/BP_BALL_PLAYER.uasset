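; Player ball pawn, an early physics-driven prototype with mouse-look style Turn and LookUp axes feeding controller yaw and pitch.
; Pressing W restarts a timeline, and only when it finishes does the PLAYER component receive one impulse at the actor's location from the timeline's Impulse track.
; MoveForward and MoveRight axis events are empty, with their AddMovementInput nodes and a MultiGate left disconnected.
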(event `InputAxis|Turn`
  (params (AxisValue :type "Float (single-precision)"))
  (`self.AddControllerYawInput` AxisValue))

(event `InputAxis|LookUp`
  (params (AxisValue :type "Float (single-precision)"))
  (`self.AddControllerPitchInput` AxisValue))

(event `Key|W`
  (params (Key :type "Key Structure"))
  (:`Pressed`
    (bind (_direction _impulse) (`Timeline|Timeline_0` :!via `PlayFromStart`)
      (:`Finished`
        (`PrimitiveComponent.AddImpulseAtLocation` (`self.PLAYER`) _impulse (`self.K2_GetActorLocation`) "None")))))

(event `InputAxis|MoveForward`
  (params (AxisValue :type "Float (single-precision)")))

(event `InputAxis|MoveRight`
  (params (AxisValue :type "Float (single-precision)")))

(fn `UserConstructionScript`)